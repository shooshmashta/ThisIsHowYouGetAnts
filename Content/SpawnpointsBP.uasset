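; Spawn point actor that registers itself with the game mode so it can be used for spawning.
; On BeginPlay it destroys itself if its Y location is 510 or beyond, otherwise it adds itself to MainGameMode's SpawnPoints array.
; It also destroys itself whenever another actor overlaps it.
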(event `self.ReceiveBeginPlay`
  (if (>= (.y (.location (`self.GetTransform`))) 510.0)
    (`self.K2_DestroyActor`)
    (else
      (bind _asmain_game_mode (cast `/Game/MainGameMode` (`GameplayStatics.GetGameMode`)))
      (`KismetArrayLibrary.Array_Add` (`/Game/MainGameMode.SpawnPoints` _asmain_game_mode) self))))

(event `self.ReceiveActorBeginOverlap`
  (params (OtherActor :type "Actor Object Reference"))
  (`self.K2_DestroyActor`))

(event `self.ReceiveTick`
  (params (DeltaSeconds :type "Float (single-precision)")))

(fn `UserConstructionScript`)